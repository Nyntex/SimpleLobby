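; Player state Blueprint that holds a player's chosen Faction and Spawnpoint.
; RPC_Server_UpdateSettings forwards both values to RPC_UpdateSettings, which stores them on the player state.
; It then records the spawnpoint in BP_GameInstance's PlayerSpawnpoints map under the PlayerId and calls the SettingsChanged dispatcher, provided the game instance cast succeeds.
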(event `self.ReceiveBeginPlay`)

(event `RPC_Server_UpdateSettings`
  (params (Faction :type "/Game/Player/EFactions Enum" :default "NewEnumerator0") (Spawnpoint :type Integer))
  (`self.RPC_UpdateSettings` Faction Spawnpoint))

(event `RPC_UpdateSettings`
  (params (Faction :type "/Game/Player/EFactions Enum" :default "NewEnumerator0") (Spawnpoint :type Integer))
  (set `self.Faction` Faction)
  (set `self.Spawnpoint` Spawnpoint)
  (bind _asbp_game_instance (cast `/Game/GeneralLogic/BP_GameInstance` (`GameplayStatics.GetGameInstance`)))
  (`BlueprintMapLibrary.Map_Add` (`/Game/GeneralLogic/BP_GameInstance.PlayerSpawnpoints` _asbp_game_instance) (`self.PlayerId`) (`self.Spawnpoint`))
  (`self.SettingsChanged`))

(fn `UserConstructionScript`)